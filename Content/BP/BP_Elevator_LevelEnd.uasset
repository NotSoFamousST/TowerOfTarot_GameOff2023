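; Level-end elevator trigger that lets the player finish the current area (Atrium, Boiler Room or Living Quarters) once its enemies are cleared.
; Player overlap checks the EnemyManager's remaining count for the current level, flashing the enemies-remaining widget if any are left.
; Otherwise, it closes the referenced elevator's doors, plays movement audio after a delay, sets NextLevel on the manager and fades to black.
; It also closes the doors on overlap end after completion.
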(event OnComponentBeginOverlap(Col)
  (params (OverlappedComponent :type Primitive%20Component%20Object%20Reference) (OtherActor :type Actor%20Object%20Reference) (OtherComp :type Primitive%20Component%20Object%20Reference) (OtherBodyIndex :type Integer) (bFromSweep :type Boolean) (SweepResult :type Hit%20Result%20Structure%20%28by%20ref%29))
  (bind _enemy_manager (Variables|Default|GetEnemy%20manager))
  (if (Actor|ActorHasTag OtherActor "Player")
    (if (== (Utilities|Select :Index (Variables|/Game/BP/BP_enemyManager.BP_enemyManager_C|GetCurrent%20Level _enemy_manager) :NewEnumerator0 (Variables|/Game/BP/BP_enemyManager.BP_enemyManager_C|GetRemaining%20Atrium%20Enemy%20Count _enemy_manager) :NewEnumerator1 (Variables|/Game/BP/BP_enemyManager.BP_enemyManager_C|GetRemaining%20Boiler%20Enemy%20Count _enemy_manager) :NewEnumerator2 (Variables|/Game/BP/BP_enemyManager.BP_enemyManager_C|GetRemaining%20Living%20Enemy%20Count _enemy_manager)) 0)
      (Utilities|FlowControl|DoOnce false
        (:Completed
          (CallFunction|EndLevel)))
      (else
        (bind _foundwidgets (Widget|GetAllWidgetsOfClass "/Game/UI/UI_EnemiesRemaining.UI_EnemiesRemaining_C" true))
        (Default|FlashText (Utilities|Array|Get(acopy) _foundwidgets))))))

(event OnComponentEndOverlap(Col)
  (params (OverlappedComponent :type Primitive%20Component%20Object%20Reference) (OtherActor :type Actor%20Object%20Reference) (OtherComp :type Primitive%20Component%20Object%20Reference) (OtherBodyIndex :type Integer))
  (if (Variables|Default|GetClose%20elevator%20after%20leaving)
    (Default|CloseElevatorDoors (Variables|Default|GetElevator%20Ref))))

(event Custom|End%20level
  (bind _elevator_ref (Variables|Default|GetElevator%20Ref))
  (Default|CloseElevatorDoors _elevator_ref)
  (Utilities|FlowControl|Delay 3.0)
  (Audio|Components|Audio|Play (Variables|/Game/BP/BP_Elevator.BP_Elevator_C|GetAudioComp_Movement _elevator_ref) 0.0)
  (Variables|/Game/BP/BP_enemyManager.BP_enemyManager_C|SetCurrent%20Level (Variables|Default|GetEnemy%20manager) (Variables|Default|GetNext%20Level))
  (Variables|Default|SetClose%20elevator%20after%20leaving true)
  (bind _returnvalue (UserInterface|CreateWidget "/Game/UI/UI_FadeToBlack.UI_FadeToBlack_C" (Game|GetPlayerController 0)))
  (UserInterface|Viewport|AddtoViewport _returnvalue 0)
  (Default|FadeAnim _returnvalue true)
  (bind _foundwidgets (Widget|GetAllWidgetsOfClass "/Game/UI/UI_EnemiesRemaining.UI_EnemiesRemaining_C" true))
  (Default|SetTexttoKillEnemiesText (Utilities|Array|Get(acopy) _foundwidgets)))

(fn ConstructionScript)