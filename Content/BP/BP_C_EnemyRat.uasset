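; Enemy rat character that chases the first-person player on sight and damages them on overlap with its box.
; PawnSensing triggers AIMoveTo toward the player and a one-time start of the rat loop audio.
; Incoming damage updates clamped health and its widget bar, which a looping timer yaws toward the player.
; At zero health the actor is destroyed immediately, leaving the ragdoll and delayed-destroy nodes disconnected.
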(event OnSeePawn(PawnSensing)
  (params (Pawn :type Pawn%20Object%20Reference))
  (bind _asbp_first_person_character (Utilities|Casting|CastToBP_FirstPersonCharacter Pawn))
  (AI|AIMoveTo self "0, 0, 0" _asbp_first_person_character 5.0 false
    (:then
      (Utilities|FlowControl|DoOnce false
        (:Completed
          (Audio|Components|Audio|Play (Variables|Default|GetAudio_Comp_Rat_Loop) 0.0))))))

(event OnComponentBeginOverlap(Box)
  (params (OverlappedComponent :type Primitive%20Component%20Object%20Reference) (OtherActor :type Actor%20Object%20Reference) (OtherComp :type Primitive%20Component%20Object%20Reference) (OtherBodyIndex :type Integer) (bFromSweep :type Boolean) (SweepResult :type Hit%20Result%20Structure%20%28by%20ref%29))
  (bind _asbp_first_person_character (Utilities|Casting|CastToBP_FirstPersonCharacter OtherActor))
  (Game|Damage|ApplyDamage _asbp_first_person_character 1.0 0 self))

(event Custom|Face%20health%20bar%20towards%20player
  (bind _health_widget (Variables|Default|GetHealth%20Widget))
  ;[1 1 1] Rotate health bar towards player camera
  (Transformation|SetWorldRotation _health_widget (Math|Rotator|MakeRotator 0.0 0.0 (.yaw (Math|Rotator|FindLookatRotation (Transformation|GetWorldLocation _health_widget) (Transformation|GetActorLocation (Game|GetPlayerCharacter 0))))) false false))

(event Custom|Update%20health%20bar
  ;[1 1 1] Update health bar widget
  (bind _asui_enemy_health (Utilities|Casting|CastToUI_Enemy_Health (UserInterface|GetWidget (Variables|Default|GetHealth%20Widget))))
  (Progress|SetPercent (Variables|/Game/UI/UI_Enemy_Health.UI_Enemy_Health_C|GetPB_Health _asui_enemy_health) (/ (Variables|Default|GetCurrent%20Health) 1e+02)))

(event Custom|Death
  ;[1 1 1] Enemy death
  (Actor|DestroyActor))

(event EventBeginPlay
  ;[1 1 1] Init
  (Utilities|Time|SetTimerbyFunctionName 0 "Face health bar towards player" 0.1 true))

(event Game|Damage|EventAnyDamage
  (params (Damage :type Float%20%28single-precision%29) (DamageType :type Damage%20Type%20Object%20Reference) (InstigatedBy :type Controller%20Object%20Reference) (DamageCauser :type Actor%20Object%20Reference))
  ;[1 1 1] Take damage
  (Variables|Default|SetCurrent%20Health (Math|Integer|Clamp(Integer) (Math|Float|Truncate (- (Variables|Default|GetCurrent%20Health) Damage)) 0 100))
  (CallFunction|UpdateHealthBar)
  (if (<= (Variables|Default|GetCurrent%20Health) 0)
    (CallFunction|Death)))

(fn ConstructionScript)