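; Floating eye enemy that shoots the player on sight, blinks on a randomized delay and shatters into BP_DestructiblePeepo on death.
; PawnSensing turns it toward the player and fires projectiles with a one-second cooldown.
; Damage updates a health bar widget, which a looping timer yaws toward the player.
; BeginPlay caches three patrol points and picks one at random, but the Patrol timeline that would move between them is never started.
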(event OnSeePawn(PawnSensing)
  (params (Pawn :type Pawn%20Object%20Reference))
  ;[1 1 1] Shoot at Player
  (bind _asbp_first_person_character (Utilities|Casting|CastToBP_FirstPersonCharacter Pawn))
  (Utilities|FlowControl|Sequence
    (:then_0
      (Transformation|SetActorRotation (Math|Rotator|FindRelativeLookatRotation (Math|Conversions|ToTransform(Vector) (Transformation|GetActorLocation)) (Transformation|GetActorLocation _asbp_first_person_character))))
    (:then_1
      (if (Variables|Default|GetSpawnProjectile)
        (Audio|Components|Audio|Play (Variables|Default|GetAudio_Comp_Shoot) 0.0)
        (Game|SpawnActorfromClass "/Game/FirstPerson/Blueprints/BP_EnemyProjectile.BP_EnemyProjectile_C" (Transformation|GetWorldTransform (Variables|Default|GetSpawnBullet)) "Undefined" 0 0)
        (Variables|Default|SetSpawnProjectile false)
        (Utilities|FlowControl|Delay 1.0)
        (Variables|Default|SetSpawnProjectile true)))))

(event Custom|Face%20health%20bar%20towards%20player
  (bind _health_widget (Variables|Default|GetHealth%20Widget))
  ;[1 1 1] Rotate health bar towards player camera
  (Transformation|SetWorldRotation _health_widget (Math|Rotator|MakeRotator 0.0 0.0 (.yaw (Math|Rotator|FindLookatRotation (Transformation|GetWorldLocation _health_widget) (Transformation|GetActorLocation (Game|GetPlayerCharacter 0))))) false false))

(event Custom|Update%20health%20bar
  ;[1 1 1] Update health bar widget
  (bind _asui_enemy_health (Utilities|Casting|CastToUI_Enemy_Health (UserInterface|GetWidget (Variables|Default|GetHealth%20Widget))))
  (Progress|SetPercent (Variables|/Game/UI/UI_Enemy_Health.UI_Enemy_Health_C|GetPB_Health _asui_enemy_health) (/ (Variables|Default|GetCurrent%20Health) (Variables|Default|GetMax%20Health))))

(event Custom|Death
  ;[1 1 1] Enemy death
  (Game|SpawnActorfromClass "/Game/BP/BP_DestructiblePeepo.BP_DestructiblePeepo_C" (Transformation|GetWorldTransform (Variables|Default|GetEyeModel)) "Undefined" 0 0)
  (Actor|DestroyActor))

(event Custom|Blink%20at%20random%20intervals
  (Utilities|FlowControl|Delay (Math|Random|RandomFloatinRange 1.0 3.0))
  (Components|Animation|PlayAnimation (Variables|Default|GetInner_Eye) "/Game/Animation/Enemy/Eye_Enemy/Anims/Eye_Anim_Blink.Eye_Anim_Blink" false))

(event EventBeginPlay
  ;[1 1 1] Init
  (Utilities|FlowControl|Sequence
    (:then_0
      (Utilities|Time|SetTimerbyFunctionName 0 "Face health bar towards player" 0.1 true))
    (:then_1
      (Variables|Default|SetPatrolPoints (Utilities|Array|MakeArray (Transformation|GetWorldLocation (Variables|Default|GetMovepos1)) (Transformation|GetWorldLocation (Variables|Default|GetMovepos2)) (Transformation|GetWorldLocation (Variables|Default|GetMovepos3))))
      (CallFunction|GetRandomLoc))
    (:then_2
      (Utilities|Time|SetTimerbyFunctionName 0 "Blink at random intervals" 1.0 true))
    (:then_3
      (Audio|Components|Audio|Play (Variables|Default|GetAudio_Comp_Hover) 0.0))))

(event Game|Damage|EventAnyDamage
  (params (Damage :type Float%20%28single-precision%29) (DamageType :type Damage%20Type%20Object%20Reference) (InstigatedBy :type Controller%20Object%20Reference) (DamageCauser :type Actor%20Object%20Reference))
  ;[1 1 1] Take damage
  (Variables|Default|SetCurrent%20Health (Math|Integer|Clamp(Integer) (Math|Float|Truncate (- (Variables|Default|GetCurrent%20Health) Damage)) 0 100))
  (CallFunction|UpdateHealthBar)
  (if (<= (Variables|Default|GetCurrent%20Health) 0)
    (CallFunction|Death)
    (else
      (Rendering|SetVisibility (Variables|Default|GetHealth%20Widget) true false))))

(fn ConstructionScript)

(fn GetRandomLoc
  (Variables|Default|SetCurrentPatrolPoint (Math|Random|RandomInteger (Utilities|Array|Length (Variables|Default|GetPatrolPoints)))))