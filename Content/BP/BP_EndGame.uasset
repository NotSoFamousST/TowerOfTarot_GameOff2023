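; BP_EndGame is a trigger actor that ends the game when an actor tagged Player overlaps its Col component.
; The overlap fires once, closes the doors on the referenced elevator, waits briefly, then plays a UI_FadeToBlack fade.
; After a further delay it adds the UI_EndGame widget to the viewport.
; BeginPlay only casts the game instance and does nothing with the result.
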(event OnComponentBeginOverlap(Col)
  (params (OverlappedComponent :type Primitive%20Component%20Object%20Reference) (OtherActor :type Actor%20Object%20Reference) (OtherComp :type Primitive%20Component%20Object%20Reference) (OtherBodyIndex :type Integer) (bFromSweep :type Boolean) (SweepResult :type Hit%20Result%20Structure%20%28by%20ref%29))
  (bind _returnvalue (Game|GetPlayerController 0))
  (if (Actor|ActorHasTag OtherActor "Player")
    (Utilities|FlowControl|DoOnce false
      (:Completed
        (Default|CloseElevatorDoors (Variables|Default|GetElevator%20Ref))
        (Utilities|FlowControl|Delay 1.0)
        (bind _returnvalue_2 (UserInterface|CreateWidget "/Game/UI/UI_FadeToBlack.UI_FadeToBlack_C" _returnvalue))
        (UserInterface|Viewport|AddtoViewport _returnvalue_2 0)
        (Default|FadeAnim _returnvalue_2 true)
        (Utilities|FlowControl|Delay 2.0)
        (bind _returnvalue_3 (UserInterface|CreateWidget "/Game/UI/UI_EndGame.UI_EndGame_C" _returnvalue))
        (UserInterface|Viewport|AddtoViewport _returnvalue_3 0)))))

(event EventBeginPlay
  (Utilities|Casting|CastToGameInstance (Game|GetGameInstance)))

(fn ConstructionScript)