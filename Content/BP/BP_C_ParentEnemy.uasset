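; Parent enemy character Blueprint handling health, damage feedback and death.
; Damage updates and reveals a widget health bar, spawns a damage number, shows shock VFX if that component exists, and destroys the actor at zero health; ragdoll logic is unwired.
; Looping timers yaw the bar toward the player and adjust walk speed when an upgraded player drops below 50 health, though dividing by 0.75 raises speed despite the "Reduce speed" label.
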(event Custom|Face%20health%20bar%20towards%20player
  (bind _health_widget (Variables|Default|GetHealth%20Widget))
  ;[1 1 1] Rotate health bar towards player camera
  (Transformation|SetWorldRotation _health_widget (Math|Rotator|MakeRotator 0.0 0.0 (.yaw (Math|Rotator|FindLookatRotation (Transformation|GetWorldLocation _health_widget) (Transformation|GetActorLocation (Game|GetPlayerCharacter 0))))) false false))

(event Custom|Update%20health%20bar
  ;[1 1 1] Update health bar widget
  (bind _asui_enemy_health (Utilities|Casting|CastToUI_Enemy_Health (UserInterface|GetWidget (Variables|Default|GetHealth%20Widget))))
  (Progress|SetPercent (Variables|/Game/UI/UI_Enemy_Health.UI_Enemy_Health_C|GetPB_Health _asui_enemy_health) (/ (Variables|Default|GetCurrent%20Health) 1e+02)))

(event Custom|Death
  ;[1 1 1] Enemy death
  (Actor|DestroyActor))

(event Custom|Show%20damage%20amount
  (params (Damage%20Amount :type Float%20%28double-precision%29))
  (bind _returnvalue (Game|SpawnActorfromClass "/Game/BP/BP_DamageIndicator.BP_DamageIndicator_C" (Math|Transform|MakeTransform (Transformation|GetWorldLocation (Variables|Default|GetDamageValueSpawn)) "0, 0, 0" "1.000000,1.000000,1.000000") "Undefined" 0 0))
  (bind _asui_damage_value (Utilities|Casting|CastToUI_DamageValue (UserInterface|GetWidget (Variables|/Game/BP/BP_DamageIndicator.BP_DamageIndicator_C|GetDamage%20Value _returnvalue))))
  (Default|ShowDamage _asui_damage_value Damage%20Amount))

(event Custom|Check%20player%20health
  (bind _player_ref (Variables|Default|GetPlayer%20Ref))
  (bind _charactermovement (Variables|Character|GetCharacterMovement))
  (bind _default_walk_speed (Variables|Default|GetDefault%20Walk%20Speed))
  ;[1 1 1] Check player health nad reduce speed if health is below 50% + player has respective upgrade
  (if (and (Variables|/Game/FirstPerson/Blueprints/BP_FirstPersonCharacter.BP_FirstPersonCharacter_C|GetHas%20reduced%20enemy%20speed _player_ref) (< (Variables|/Game/FirstPerson/Blueprints/BP_FirstPersonCharacter.BP_FirstPersonCharacter_C|GetCurrent%20Health _player_ref) 50))
    (Variables|/Script/Engine.CharacterMovementComponent|SetMaxWalkSpeed _charactermovement (/ _default_walk_speed 0.75))
    (Development|PrintString "Reduce speed")
    (else
      (Variables|/Script/Engine.CharacterMovementComponent|SetMaxWalkSpeed _charactermovement _default_walk_speed))))

(event EventBeginPlay
  (bind _asbp_first_person_character (Utilities|Casting|CastToBP_FirstPersonCharacter (Game|GetPlayerCharacter 0)))
  ;[1 1 1] Init
  (Variables|Default|SetPlayer%20Ref _asbp_first_person_character)
  (Variables|Default|SetDefault%20Walk%20Speed (Variables|/Script/Engine.CharacterMovementComponent|GetMaxWalkSpeed (Variables|Character|GetCharacterMovement)))
  (Utilities|Time|SetTimerbyFunctionName 0 "Face health bar towards player" 0.1 true)
  (Utilities|Time|SetTimerbyFunctionName 0 "Check player health" 0.2 true))

(event Game|Damage|EventAnyDamage
  (params (Damage :type Float%20%28single-precision%29) (DamageType :type Damage%20Type%20Object%20Reference) (InstigatedBy :type Controller%20Object%20Reference) (DamageCauser :type Actor%20Object%20Reference))
  ;[1 1 1] Take damage
  (Rendering|SetVisibility (Variables|Default|GetHealth%20Widget) true false)
  (Variables|Default|SetCurrent%20Health (Math|Integer|Clamp(Integer) (Math|Float|Truncate (- (Variables|Default|GetCurrent%20Health) Damage)) 0 (Variables|Default|GetMax%20Health)))
  (CallFunction|UpdateHealthBar)
  (CallFunction|ShowDamageAmount Damage)
  (if (<= (Variables|Default|GetCurrent%20Health) 0)
    (CallFunction|Death)
    (else
      (Utilities|IsValid (Actor|GetComponentbyClass "/Game/BP/BPC_ShockDamage.BPC_ShockDamage_C")
        (:Is%20Valid
          (Rendering|SetVisibility (Variables|Default|GetShockDMG) true false))))))

(fn ConstructionScript)