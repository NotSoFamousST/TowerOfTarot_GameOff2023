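; Grenade launcher projectile that explodes when it gets close to a surface.
; Each tick a short Visibility trace runs forward from the Grenade component, standing in for collision events.
; The first hit plays the impact sound, deals full radial damage that spares player character 0, and spawns an explosion effect.
; The effect and actor are destroyed after a short delay.
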(event EventBeginPlay)

(event Collision|EventActorBeginOverlap
  (params (OtherActor :type Actor%20Object%20Reference)))

(event EventTick
  (params (DeltaSeconds :type Float%20%28single-precision%29))
  (bind _returnvalue (Transformation|GetActorLocation))
  (bind _grenade (Variables|Default|GetGrenade))
  (bind _returnvalue_2 (Transformation|GetWorldLocation _grenade))
  (bind _returnvalue_3 (Collision|LineTraceByChannel _returnvalue_2 (+ _returnvalue_2 (* (Math|Vector|GetForwardVector _grenade) 1e+02)) "TraceTypeQuery1" false 0 "None"))
  (if _returnvalue_3
    (Utilities|FlowControl|DoOnce false
      (:Completed
        (Audio|PlaySoundatLocation "/Game/Audio/Game_Audio/Audio_Setups/Weapon_MetaSound/sfx_meta_grenade_impact.sfx_meta_grenade_impact" (Transformation|GetActorLocation) "0, 0, 0" 1.0 1.0 0.0 0 0 0 0)
        (Game|Damage|ApplyRadialDamage (Variables|Default|GetExplosion%20Damage) _returnvalue 2.5e+02 0 (Utilities|Array|MakeArray (Game|GetPlayerCharacter 0)) self 0 true "ECC_Visibility")
        (bind _returnvalue_4 (Effects|SpawnEmitteratLocation "/Game/FX/P_Explosion.P_Explosion" _returnvalue "0, 0, 0" "2.000000,2.000000,2.000000"))
        (Utilities|FlowControl|Delay 1.0)
        (Components|DestroyComponent _returnvalue_4)
        (Actor|DestroyActor)))))

(fn ConstructionScript)