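; BP_Col_AssignEnemiesToLevel is a collision volume that registers enemies to a level area.
; On BeginPlay it caches the first BP_enemyManager found in the world.
; When an actor tagged "Enemy" begins overlapping the collision, a switch on its Level value adds that actor uniquely to the manager's Atrium, Boiler Room or Living Quarters enemy array.
; The Atrium branch also prints a debug string.
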(event OnComponentBeginOverlap(Col)
  (params (OverlappedComponent :type Primitive%20Component%20Object%20Reference) (OtherActor :type Actor%20Object%20Reference) (OtherComp :type Primitive%20Component%20Object%20Reference) (OtherBodyIndex :type Integer) (bFromSweep :type Boolean) (SweepResult :type Hit%20Result%20Structure%20%28by%20ref%29))
  (bind _enemy_manager_ref (Variables|Default|GetEnemy%20Manager%20Ref))
  (if (Actor|ActorHasTag OtherActor "Enemy")
    (switch Utilities|FlowControl|Switch|SwitchonEnum_CurrentLevel (Variables|Default|GetLevel)
      (:NewEnumerator0
        (Utilities|Array|AddUnique (Variables|/Game/BP/BP_enemyManager.BP_enemyManager_C|GetAtrium%20Enemies _enemy_manager_ref) OtherActor)
        (Development|PrintString "Hello"))
      (:NewEnumerator1
        (Utilities|Array|AddUnique (Variables|/Game/BP/BP_enemyManager.BP_enemyManager_C|GetBoiler%20room%20Enemies _enemy_manager_ref) OtherActor))
      (:NewEnumerator2
        (Utilities|Array|AddUnique (Variables|/Game/BP/BP_enemyManager.BP_enemyManager_C|GetLiving%20Quarters%20Enemies _enemy_manager_ref) OtherActor)))))

(event EventBeginPlay
  (bind _outactors (Actor|GetAllActorsOfClass "/Game/BP/BP_enemyManager.BP_enemyManager_C"))
  (Variables|Default|SetEnemy%20Manager%20Ref (Utilities|Array|Get(acopy) _outactors)))

(fn ConstructionScript)