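; Base interactable actor, judging by its name, with placeholder interact, show and hide events that print debug messages.
; Show and hide swap the object's material between emissive green and red.
; Each is gated by a DoOnce that the opposite event resets, so repeated calls fire only once.
; A fast looping timer started on BeginPlay yaws the debug TextRender toward the player character.
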(event Custom|Face%20debug%20text%20towards%20player
  (bind _textrender (Variables|Default|GetTextRender))
  (Transformation|SetWorldRotation _textrender (Math|Rotator|MakeRotator 0.0 0.0 (.yaw (Math|Rotator|FindLookatRotation (Transformation|GetWorldLocation _textrender) (Transformation|GetActorLocation (Game|GetPlayerCharacter 0))))) false false))

(event Custom|Reset%20show%20interaction
  (Utilities|FlowControl|DoOnce false) ; enters at Reset
)

(event Custom|Reset%20hide%20interaction
  (Utilities|FlowControl|DoOnce false) ; enters at Reset
)

(event EventBeginPlay
  (Utilities|Time|SetTimerbyFunctionName 0 "Face debug text towards player" 0.02 true))

(event EventFireInteraction
  (Development|PrintString "Actor interacted with" true true "(R=0.000000,G=0.660000,B=1.000000,A=1.000000)" 1.0))

(event EventHideInteraction
  (Utilities|FlowControl|DoOnce false
    (:Completed
      (Rendering|Material|SetMaterial (Variables|Default|GetObject) 0 "/Game/Materials/M_Red.M_Red")
      (CallFunction|ResetShowInteraction)
      (Development|PrintString "Hide interaction" true true "(R=1.000000,G=0.007579,B=0.000000,A=1.000000)" 1.0))))

(event EventShowInteraction
  (Utilities|FlowControl|DoOnce false
    (:Completed
      (Rendering|Material|SetMaterial (Variables|Default|GetObject) 0 "/Game/Materials/M_Emissive_Green.M_Emissive_Green")
      (CallFunction|ResetHideInteraction)
      (Development|PrintString "Show interaction" true true "(R=0.014199,G=1.000000,B=0.000000,A=1.000000)" 1.0))))

(fn ConstructionScript)