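; BP_enemyManager tracks how many enemies remain in the Atrium, Boiler and Living levels and updates the UI when one is cleared.
; A fast looping timer started on BeginPlay polls the actors carrying each level's tag and stores the count per level.
; When a count reaches zero, that level's DoOnce switches the first top-level UI_EnemiesRemaining widget to its find-elevator text.
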(event Custom|Check%20enemies%20left
  (Utilities|FlowControl|Sequence
    (:then_0
      (bind _outactors (Actor|GetAllActorswithTag "Level_Atrium"))
      (bind _output_get (Variables|Default|SetRemaining%20Atrium%20Enemy%20Count (Utilities|Array|Length _outactors)))
      (if (== _output_get 0)
        (Utilities|FlowControl|DoOnce false
          (:Completed
            (bind _foundwidgets (Widget|GetAllWidgetsOfClass "/Game/UI/UI_EnemiesRemaining.UI_EnemiesRemaining_C" true :!label _label))
            (Default|SetTexttoFindElevatorText (Utilities|Array|Get(acopy) _foundwidgets))))))
    (:then_1
      (bind _outactors_2 (Actor|GetAllActorswithTag "Level_Boiler"))
      (bind _output_get_2 (Variables|Default|SetRemaining%20Boiler%20Enemy%20Count (Utilities|Array|Length _outactors_2)))
      (if (== _output_get_2 0)
        (Utilities|FlowControl|DoOnce false
          (:Completed
            (goto _label)))))
    (:then_2
      (bind _outactors_3 (Actor|GetAllActorswithTag "Level_Living"))
      (bind _output_get_3 (Variables|Default|SetRemaining%20Living%20Enemy%20Count (Utilities|Array|Length _outactors_3)))
      (if (== _output_get_3 0)
        (Utilities|FlowControl|DoOnce false
          (:Completed
            (goto _label)))))))

(event EventBeginPlay
  (Utilities|Time|SetTimerbyEvent (delegate Custom|Check%20enemies%20left) 0.1 true))

(fn ConstructionScript)