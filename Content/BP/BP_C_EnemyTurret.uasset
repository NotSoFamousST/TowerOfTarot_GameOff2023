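; Enemy turret that turns to face the player on sight and fires projectiles at them.
; Pawn sensing drives the rotation and spawns BP_EnemyProjectile with a shot sound, throttled by a flag and delay.
; BeginPlay starts a hover sound and a looping timer for health bar facing, but that event is empty.
; Damage, health bar update and ragdoll death logic exist only as disconnected nodes, leaving those events empty.
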(event OnSeePawn(PawnSensing)
  (params (Pawn :type Pawn%20Object%20Reference))
  (bind _asbp_first_person_character (Utilities|Casting|CastToBP_FirstPersonCharacter Pawn))
  (Utilities|FlowControl|Sequence
    (:then_0
      (Transformation|SetActorRotation (Math|Rotator|FindRelativeLookatRotation (Math|Conversions|ToTransform(Vector) (Transformation|GetActorLocation)) (Transformation|GetActorLocation _asbp_first_person_character))))
    (:then_1
      (if (Variables|Default|GetSpawnProjectile)
        (Audio|Components|Audio|Play (Variables|Default|GetAudio_Comp_Shoot) 0.0)
        (Game|SpawnActorfromClass "/Game/FirstPerson/Blueprints/BP_EnemyProjectile.BP_EnemyProjectile_C" (Transformation|GetWorldTransform (Variables|Default|GetSpawnBullet)) "Undefined" 0 0)
        (Variables|Default|SetSpawnProjectile false)
        (Utilities|FlowControl|Delay 1.0)
        (Variables|Default|SetSpawnProjectile true)))))

(event Custom|Face%20health%20bar%20towards%20player
  ;[1 1 1] Rotate health bar towards player camera
)

(event Custom|Update%20health%20bar
  ;[1 1 1] Update health bar widget
)

(event Custom|Death
  ;[1 1 1] Enemy death
)

(event EventBeginPlay
  ;[1 1 1] Init
  (Utilities|Time|SetTimerbyFunctionName 0 "Face health bar towards player" 0.1 true)
  (Audio|Components|Audio|Play (Variables|Default|GetAudio_Comp_Hover) 0.0))

(event Game|Damage|EventAnyDamage
  (params (Damage :type Float%20%28single-precision%29) (DamageType :type Damage%20Type%20Object%20Reference) (InstigatedBy :type Controller%20Object%20Reference) (DamageCauser :type Actor%20Object%20Reference))
  ;[1 1 1] Take damage
)

(fn ConstructionScript)