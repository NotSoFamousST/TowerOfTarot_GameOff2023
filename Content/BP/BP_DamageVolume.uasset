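; BP_DamageVolume is a volume actor that applies DamageAmount damage to an overlapping actor tagged Player.
; A DoOnce gate makes the damage fire once per entry and resets when the player's overlap ends.
; A looping fast timer calls an event that yaws the DebugName text to face the first player character.
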(event OnComponentBeginOverlap(DamageVolume)
  (params (OverlappedComponent :type Primitive%20Component%20Object%20Reference) (OtherActor :type Actor%20Object%20Reference) (OtherComp :type Primitive%20Component%20Object%20Reference) (OtherBodyIndex :type Integer) (bFromSweep :type Boolean) (SweepResult :type Hit%20Result%20Structure%20%28by%20ref%29))
  (if (Actor|ActorHasTag OtherActor "Player")
    (Utilities|FlowControl|DoOnce false
      (:Completed
        (Game|Damage|ApplyDamage OtherActor (Variables|Default|GetDamage%20Amount) 0 self)))))

(event OnComponentEndOverlap(DamageVolume)
  (params (OverlappedComponent :type Primitive%20Component%20Object%20Reference) (OtherActor :type Actor%20Object%20Reference) (OtherComp :type Primitive%20Component%20Object%20Reference) (OtherBodyIndex :type Integer))
  (if (Actor|ActorHasTag OtherActor "Player")
    (Utilities|FlowControl|DoOnce false) ; enters at Reset
  ))

(event Custom|Face%20debug%20text%20towards%20player
  (bind _debug_name (Variables|Default|GetDebug%20Name))
  (Transformation|SetWorldRotation _debug_name (Math|Rotator|MakeRotator 0.0 0.0 (.yaw (Math|Rotator|FindLookatRotation (Transformation|GetWorldLocation _debug_name) (Transformation|GetActorLocation (Game|GetPlayerCharacter 0))))) false false))

(event EventBeginPlay
  (Utilities|Time|SetTimerbyFunctionName 0 "Face debug text towards player" 0.02 true))

(fn ConstructionScript)