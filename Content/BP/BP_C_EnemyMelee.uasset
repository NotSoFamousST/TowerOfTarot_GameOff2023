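; Melee enemy character that chases the first-person player when pawn sensing spots them and damages them when its box trigger overlaps them.
; A looping timer yaws the health bar widget toward the player; taking damage updates and reveals it.
; Movement and attack audio accompany chasing and hits.
; At zero health it disables sensing, pawn collision and audio, plays a dying animation, then destroys itself after a delay.
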(event OnSeePawn(PawnSensing)
  (params (Pawn :type Pawn%20Object%20Reference))
  (bind _asbp_first_person_character (Utilities|Casting|CastToBP_FirstPersonCharacter Pawn))
  (AI|AIMoveTo self "0, 0, 0" _asbp_first_person_character 5.0 false
    (:then
      ;[1 1 1] Activate Audio of cc Enemy Do Once if running attack if cc
      (Utilities|FlowControl|DoOnce false :!label _label
        (:Completed
          (Audio|Components|Audio|Play (Variables|Default|GetAuido_Comp_CC_Movement) 0.0))))
    (:OnSuccess
      (Class|AudioParameterControllerInterface|SetTriggerParameter (Variables|Default|GetAuido_Comp_CC_Movement) "Stop_running")
      (goto _label Reset))))

(event OnComponentBeginOverlap(Box)
  (params (OverlappedComponent :type Primitive%20Component%20Object%20Reference) (OtherActor :type Actor%20Object%20Reference) (OtherComp :type Primitive%20Component%20Object%20Reference) (OtherBodyIndex :type Integer) (bFromSweep :type Boolean) (SweepResult :type Hit%20Result%20Structure%20%28by%20ref%29))
  (bind _asbp_first_person_character (Utilities|Casting|CastToBP_FirstPersonCharacter OtherActor))
  (Game|Damage|ApplyDamage _asbp_first_person_character (Variables|Default|GetBase%20Damage) 0 self)
  (Utilities|FlowControl|Sequence
    (:then_0
      _)
    (:then_4
      _))
  (Audio|Components|Audio|Play (Variables|Default|GetAudioComp_Attack) 0.0))

(event Custom|Face%20health%20bar%20towards%20player
  (bind _health_widget (Variables|Default|GetHealth%20Widget))
  ;[1 1 1] Rotate health bar towards player camera
  (Transformation|SetWorldRotation _health_widget (Math|Rotator|MakeRotator 0.0 0.0 (.yaw (Math|Rotator|FindLookatRotation (Transformation|GetWorldLocation _health_widget) (Transformation|GetActorLocation (Game|GetPlayerCharacter 0))))) false false))

(event Custom|Update%20health%20bar
  ;[1 1 1] Update health bar widget
  (bind _asui_enemy_health (Utilities|Casting|CastToUI_Enemy_Health (UserInterface|GetWidget (Variables|Default|GetHealth%20Widget))))
  (Progress|SetPercent (Variables|/Game/UI/UI_Enemy_Health.UI_Enemy_Health_C|GetPB_Health _asui_enemy_health) (/ (Variables|Default|GetCurrent%20Health) (Variables|Default|GetMax%20Health))))

(event Custom|Death
  (Utilities|FlowControl|DoOnce false
    (:Completed
      ;[1 1 1] Enemy death
      (Collision|SetCollisionResponsetoChannel (Variables|Character|GetMesh) "ECC_Pawn" "ECR_Ignore")
      (Collision|SetCollisionResponsetoChannel (Variables|Collision|GetCapsuleComponent) "ECC_Visibility" "ECR_Ignore")
      (Components|DestroyComponent (Variables|Default|GetPawnSensing))
      (Components|Movement|StopMovementImmediately (Variables|Character|GetCharacterMovement))
      (Rendering|SetVisibility (Variables|Default|GetHealth%20Widget) false false)
      (Collision|SetCollisionResponsetoChannel (Variables|Collision|GetCapsuleComponent) "ECC_Pawn" "ECR_Ignore")
      (Components|Animation|PlayAnimation (Variables|Character|GetMesh) "/Game/Animation/Enemy/Bellboy_Enemy/Anims/Dying_Backwards_mixamo_com.Dying_Backwards_mixamo_com" false)
      (Components|Activation|Deactivate (Variables|Default|GetAudioComp_Attack))
      (Utilities|FlowControl|Delay 2.0)
      (Actor|DestroyActor))))

(event EventBeginPlay
  ;[1 1 1] Init
  (Utilities|Time|SetTimerbyFunctionName 0 "Face health bar towards player" 0.1 true))

(event Game|Damage|EventAnyDamage
  (params (Damage :type Float%20%28single-precision%29) (DamageType :type Damage%20Type%20Object%20Reference) (InstigatedBy :type Controller%20Object%20Reference) (DamageCauser :type Actor%20Object%20Reference))
  ;[1 1 1] Take damage
  (Variables|Default|SetCurrent%20Health (Math|Integer|Clamp(Integer) (Math|Float|Truncate (- (Variables|Default|GetCurrent%20Health) Damage)) 0 100))
  (CallFunction|UpdateHealthBar)
  (if (<= (Variables|Default|GetCurrent%20Health) 0)
    (CallFunction|Death)
    (else
      (Rendering|SetVisibility (Variables|Default|GetHealth%20Widget) true false))))

(fn ConstructionScript)