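; Elevator actor that opens its timeline-driven sliding doors on BeginPlay and serves as an upgrade-selection transition.
; Closing the doors starts a looping camera-shake timer and, the first time, shows UI_UpgradeSelection with a reference to itself.
; Raising teleports the player to PlayerTPLOC with a fade widget, immediately and again when the MoveElevator timeline finishes and reopens the doors.
; The timeline only provides timing, as its height lerp is unconnected.
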(event Custom|Raise%20elevator
  (bind _player_tp_loc (Variables|Default|GetPlayer%20TP%20LOC))
  (bind _arrowcomponent (Variables|/Script/Engine.TargetPoint|GetArrowComponent _player_tp_loc))
  (bind _returnvalue (Transformation|GetWorldRotation _arrowcomponent))
  (Components|Timeline|SetPlayRate (Variables|Default|GetMove%20elevator) (Variables|Default|GetElevator%20speed))
  (Utilities|FlowControl|Sequence
    (:then_0
      (bind _alpha (Timeline|Move%20elevator Play)
        (:Finished
          (CallFunction|OpenElevatorDoors)
          (Utilities|Time|PauseTimerbyHandle (Variables|Default|GetCam%20shake%20timer))
          (Audio|Components|Audio|Stop (Variables|Default|GetAudioComp_Movement)))))
    (:then_1
      _))
  (Transformation|Teleport (Game|GetPlayerCharacter 0) (Transformation|GetActorLocation _player_tp_loc) _returnvalue)
  (Pawn|SetControlRotation (Game|GetPlayerController 0) _returnvalue)
  (bind _foundwidgets (Widget|GetAllWidgetsOfClass "/Game/UI/UI_FadeToBlack.UI_FadeToBlack_C" true))
  (Widget|RemovefromParent (Utilities|Array|Get(acopy) _foundwidgets))
  (bind _returnvalue_2 (UserInterface|CreateWidget "/Game/UI/UI_FadeToBlack.UI_FadeToBlack_C" (Game|GetPlayerController 0)))
  (Default|FadeAnim _returnvalue_2 false)
  (UserInterface|Viewport|AddtoViewport _returnvalue_2 0))

(event Custom|Open%20elevator%20doors
  (bind _doorl_initial_loc (Variables|Default|GetDoorL%20Initial%20LOC))
  (bind _doorr_initial_loc (Variables|Default|GetDoorR%20Initial%20LOC))
  (Audio|Components|Audio|Play (Variables|Default|GetAudioComp_DoorsOpen) 0.0)
  (Utilities|FlowControl|Delay 1.2)
  (bind (_direction _alpha) (Timeline|Open%20doors PlayFromStart)
    (:Update
      (Transformation|SetRelativeLocation (Variables|Default|GetDoorL) (Math|Vector|Lerp(Vector) _doorl_initial_loc (+ _doorl_initial_loc "60.000000,0.000000,0.000000") _alpha) false false)
      (Transformation|SetRelativeLocation (Variables|Default|GetDoorR) (Math|Vector|Lerp(Vector) _doorr_initial_loc (+ _doorr_initial_loc "-60.000000,0.000000,0.000000") _alpha) false false))
    (:Finished
      (switch Utilities|FlowControl|Switch|SwitchonETimelineDirection _direction
        (:Forward
          (Utilities|Time|PauseTimerbyHandle (Variables|Default|GetCam%20shake%20timer)))
        (:Backward
          (Variables|Default|SetDoors%20closed true)
          (bind _returnvalue (Utilities|Time|SetTimerbyFunctionName 0 "Elevator shake" 0.1 true))
          (Variables|Default|SetCam%20shake%20timer _returnvalue)
          (Utilities|FlowControl|DoOnce false
            (:Completed
              (Audio|PlaySound2D "/Game/Audio/Game_Audio/Audio_Setups/Menu_Meta_Sound/sfx_meta_menu_page_change.sfx_meta_menu_page_change" 5.0 1.0 0.0 0 0)
              (Utilities|FlowControl|Delay 0.2)
              (bind _returnvalue_2 (UserInterface|CreateWidget "/Game/UI/UI_UpgradeSelection.UI_UpgradeSelection_C" (Game|GetPlayerController 0) self))
              (UserInterface|Viewport|AddtoViewport _returnvalue_2 0))))))))

(event Custom|Close%20elevator%20doors
  (bind _doorl_initial_loc (Variables|Default|GetDoorL%20Initial%20LOC))
  (bind _doorr_initial_loc (Variables|Default|GetDoorR%20Initial%20LOC))
  (Audio|Components|Audio|Play (Variables|Default|GetAudioComp_DoorsClose) 0.0)
  (bind (_direction _alpha) (Timeline|Open%20doors ReverseFromEnd)
    (:Update
      (Transformation|SetRelativeLocation (Variables|Default|GetDoorL) (Math|Vector|Lerp(Vector) _doorl_initial_loc (+ _doorl_initial_loc "60.000000,0.000000,0.000000") _alpha) false false)
      (Transformation|SetRelativeLocation (Variables|Default|GetDoorR) (Math|Vector|Lerp(Vector) _doorr_initial_loc (+ _doorr_initial_loc "-60.000000,0.000000,0.000000") _alpha) false false))
    (:Finished
      (switch Utilities|FlowControl|Switch|SwitchonETimelineDirection _direction
        (:Forward
          (Utilities|Time|PauseTimerbyHandle (Variables|Default|GetCam%20shake%20timer)))
        (:Backward
          (Variables|Default|SetDoors%20closed true)
          (bind _returnvalue (Utilities|Time|SetTimerbyFunctionName 0 "Elevator shake" 0.1 true))
          (Variables|Default|SetCam%20shake%20timer _returnvalue)
          (Utilities|FlowControl|DoOnce false
            (:Completed
              (Audio|PlaySound2D "/Game/Audio/Game_Audio/Audio_Setups/Menu_Meta_Sound/sfx_meta_menu_page_change.sfx_meta_menu_page_change" 5.0 1.0 0.0 0 0)
              (Utilities|FlowControl|Delay 0.2)
              (bind _returnvalue_2 (UserInterface|CreateWidget "/Game/UI/UI_UpgradeSelection.UI_UpgradeSelection_C" (Game|GetPlayerController 0) self))
              (UserInterface|Viewport|AddtoViewport _returnvalue_2 0))))))))

(event Custom|Elevator%20shake
  (Camera|PlayWorldCameraShake "/Game/UI/CameraShakes/CamShake_Elevator.CamShake_Elevator_C" (Transformation|GetActorLocation) 5e+03 5e+03))

(event EventBeginPlay
  (Variables|Default|SetInitial%20LOC (Transformation|GetActorLocation))
  (Variables|Default|SetDoorL%20Initial%20LOC (Variables|/Script/Engine.SceneComponent|GetRelativeLocation (Variables|Default|GetDoorL)))
  (Variables|Default|SetDoorR%20Initial%20LOC (Variables|/Script/Engine.SceneComponent|GetRelativeLocation (Variables|Default|GetDoorR)))
  (CallFunction|OpenElevatorDoors))

(fn ConstructionScript)